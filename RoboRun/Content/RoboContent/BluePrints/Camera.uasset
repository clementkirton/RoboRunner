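; Camera Blueprint that auto-scrolls a camera actor each tick, switching axis by the player's movement mode, unless Testing is set.
; When not flying, it scrolls along X at fixed height as a side-scroller.
; When flying, it climbs along Z as a "TopDownScroller", with X taken once from the player's position on first flight.
; An Increase helper scales both scroll speeds by delta time; depth and rotation stay fixed.
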(event `self.ReceiveTick`
  (params (DeltaSeconds :type "Float (single-precision)"))
  (set `self.DeltaTime` DeltaSeconds)
  (if (`self.Testing`)
    _
    (elif (`NavMovementComponent.IsFlying` (`Character.CharacterMovement` (`self.Player`)))
      ;[1 1 1] TopDownScroller
      (`|ExecutionSequence`
        (:`then_0`
          (bind _out (`self.Increase` (`self.ZValue`) (`self.ZScrollerSpeed`) (`self.DeltaTime`)))
          (set `self.ZValue` _out)
          (`self.K2_SetActorTransform` (`self.Camera`) (select `bool` (`NavMovementComponent.IsFlying` (`Character.CharacterMovement` (`self.Player`))) :`false` (`KismetMathLibrary.MakeTransform` (`KismetMathLibrary.MakeVector` (stale _out_2) 2200.0 1300.0) (struct :`Yaw` -90.0)) :`true` (`KismetMathLibrary.MakeTransform` (`KismetMathLibrary.MakeVector` (`self.PlayerXSwitch`) 2200.0 _out) (struct :`Yaw` -90.0))) true false :!label _label))
        (:`then_1`
          (`/Engine/EditorBlueprintResources/StandardMacros.DoOnce` false
            (:`Completed`
              (set `self.PlayerXSwitch` (.x (.location (`self.GetTransform` (`self.Player`)))))
              (set `self.ZValue` 1300.0)))))
      (else
        ;[1 1 1] SideScroller
        (bind _out_2 (`self.Increase` (`self.XValue`) (`self.XScrollerSpeed`) (`self.DeltaTime`)))
        (set `self.XValue` _out_2)
        (goto _label)))))

(fn `Increase`
  (params (In :type "Float (double-precision)") (IncreaseAmount :type "Float (double-precision)") (TimeScale :type "Float (double-precision)" :default 1.0))
  (returns (Out :type "Float (double-precision)"))
  (return (+ In (* (* IncreaseAmount TimeScale) 100.0))))

(fn `UserConstructionScript`)